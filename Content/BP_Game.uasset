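; BP_Game is the controller of a music rhythm game, loading the first OGG song, showing the game UI and handling pause.
; A muted Tracker plays the song PLAYERDELAY ahead of the audible Player, giving low-band beat detection a lookahead.
; Tick drives the child dealer actor, skips a short window after the first detected beat, then spawns a beat on each rising edge.
; Playback end only prints a score-dialog placeholder.
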(event `self.ReceiveBeginPlay`
  (bind _asbp_game_instance (cast `/Game/BP_GameInstance` (`GameplayStatics.GetGameInstance`)))
  (set `/Game/BP_GameInstance.BP_Game_ref` self _asbp_game_instance)
  ;[1 1 1] User Interface initialization
  (bind _returnvalue (`|GenericCreateObject` "/Game/UI_Game.UI_Game_C" self))
  (bind _output_get (set `self.UI_Game` _returnvalue))
  (`/Game/UI_Game.ShowUI` _output_get)
  ;[1 1 1] To do something of playback end
  (add `AudioAnalyzerManager.OnPlaybackFinished` (`self.Player`) (delegate `OnPlaybackFinished`)))

(event `OnPlaybackFinished`
  ;[1 1 1] To do something of playback end
  (set `self.FirstDelayTriggered` false)
  (set `self.FirstDelay` 1.0)
  (`KismetSystemLibrary.PrintString` "Show score dialog"))

(event `StartAudioPlayback`
  (bind _tracker (`self.Tracker`))
  ;[1 1 1] Called from the coundown widget when reach zero
  (`AudioAnalyzerManager.SetPlaybackVolume` _tracker 0.0)
  (`AudioAnalyzerManager.Play` _tracker)
  (set `self.isPaused` false)
  (`KismetSystemLibrary.Delay` (`self.PLAYER_DELAY`))
  (`AudioAnalyzerManager.Play` (`self.Player`)))

(event `self.ReceiveTick`
  (params (DeltaSeconds :type "Float (single-precision)"))
  (if (not (`self.isPaused`))
    (set `self.DeltaTime` DeltaSeconds)
    (`self.DealersTick`)
    (bind _beats (`AudioAnalyzerManager.GetBeatTrackingWLimits` (`self.Tracker`)))
    ;[1 1 1] Discard the first seconds of the analysis
    (if (< (`self.FirstDelay`) 0.0)
      (bind _output (`|GetArrayItem` _beats))
      (`self.UpdateBeatOnSet` _output)
      (elif (`self.FirstDelayTriggered`)
        (set `self.FirstDelay` (- (`self.FirstDelay`) (`self.DeltaTime`)))
        (elif _output
          (set `self.FirstDelayTriggered` true))))))

(fn `DealersTick`
  (bind _asbp_game_dealer (cast `/Game/BP_Game_dealer` (`ChildActorComponent.ChildActor` (`self.BP_Game_dealer_0`))))
  (`/Game/BP_Game_dealer.GameTick` _asbp_game_dealer (`self.DeltaTime`)))

(fn `InitializeAudioManagers`
  ;[1 1 1] Construct AudioAnalyzerManager instances in the Game Instance
  (bind _asbp_game_instance (cast `/Game/BP_GameInstance` (`GameplayStatics.GetGameInstance`)))
  (`/Game/BP_GameInstance.InitializeGame` _asbp_game_instance)
  ;[1 1 1] Take the first audio file of the RawMusic
  (bind _asbp_game_instance_2 (cast `/Game/BP_GameInstance` (`GameplayStatics.GetGameInstance`)))
  (bind (_filenames _returnvalue) (`AudioAnalyzerManager.GetFolderFiles` (`/Game/BP_GameInstance.BP_AAManager_Player` _asbp_game_instance_2) (`KismetStringLibrary.Concat_StrStr` (`KismetSystemLibrary.GetProjectContentDirectory`) (`/Game/BP_GameInstance.RawMusicFolderName` _asbp_game_instance_2)) "ogg"))
  (if _returnvalue
    ;[1 1 1] Construct audio file path
    (bind _asbp_game_instance_3 (cast `/Game/BP_GameInstance` (`GameplayStatics.GetGameInstance`)))
    (bind _output (`|GetArrayItem` _filenames))
    (set `/Game/BP_GameInstance.SongTitle` _output _asbp_game_instance_3)
    (set `/Game/BP_GameInstance.SongPath` (`KismetStringLibrary.Concat_StrStr` (`KismetSystemLibrary.GetProjectContentDirectory`) (`/Game/BP_GameInstance.RawMusicFolderName` _asbp_game_instance_3) "/" _output) _asbp_game_instance_3)
    ;[1 1 1] Intializer dealer actor class
    (bind _asbp_game_dealer (cast `/Game/BP_Game_dealer` (`ChildActorComponent.ChildActor` (`self.BP_Game_dealer_0`))))
    (`/Game/BP_Game_dealer.InitializeDealer` _asbp_game_dealer (`self.PLAYER_DELAY`))
    ;[1 1 1] Initializes Player and Tracker and Beat Tracking analyzer
    (bind _asbp_game_instance_4 (cast `/Game/BP_GameInstance` (`GameplayStatics.GetGameInstance`)))
    (set `self.Tracker` (`/Game/BP_GameInstance.BP_AAManager_Tracker` _asbp_game_instance_4))
    (set `self.Player` (`/Game/BP_GameInstance.BP_AAManager_Player` _asbp_game_instance_4))
    (bind _songpath (`/Game/BP_GameInstance.SongPath` _asbp_game_instance_4))
    (bind _returnvalue_2 (`AudioAnalyzerManager.InitPlayerAudio` (`self.Tracker`) _songpath))
    (if _returnvalue_2
      (bind _returnvalue_3 (`AudioAnalyzerManager.InitPlayerAudio` (`self.Player`) _songpath))
      (if (not _returnvalue_3)
        (`KismetSystemLibrary.PrintString` "Init Player error"))
      (`AudioAnalyzerManager.InitBeatTrackingConfigWLimits` (`self.Tracker`) "All_in_one" 0 (`|MakeArray` (0.0 100.0) :!type "Vector2D Structure") 0.02 30 false 100 2.1)
      (else
        (`KismetSystemLibrary.PrintString` "Init Tracker error")))))

(fn `SetPause`
  (params (Pause :type Boolean))
  (bind _output_get (set `self.isPaused` Pause))
  (`AudioAnalyzerManager.SetPaused` (`self.Player`) _output_get)
  (`AudioAnalyzerManager.SetPaused` (`self.Tracker`) _output_get))

(fn `SpawnNewBeat`
  (bind _asbp_game_dealer (cast `/Game/BP_Game_dealer` (`ChildActorComponent.ChildActor` (`self.BP_Game_dealer_0`))))
  (`/Game/BP_Game_dealer.SpawnNewBeat` _asbp_game_dealer))

(fn `UpdateBeatonSet`
  (params (NewBeatState :type Boolean))
  (if (and NewBeatState (not (`self.LastBeatOnSet`)))
    (set `self.LastBeatOnSet` true)
    (`self.SpawnNewBeat`)
    (elif (and (not NewBeatState) (`self.LastBeatOnSet`))
      (set `self.LastBeatOnSet` false))))

(fn `UpdateScore`
  (params (New :type Integer))
  (`/Game/UI_Game.UpdateScore` (`self.UI_Game`) New))

(fn `UserConstructionScript`)